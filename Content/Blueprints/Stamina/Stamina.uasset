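; Character Blueprint that implements stamina-limited sprinting on Left Shift.
; Holding the key raises walk speed and drains Stamina on a looping half-second Delay; releasing it or running out restores normal speed.
; A similar Delay loop then regenerates Stamina more slowly up to MaxStamina, stopping if sprinting resumes.
; Each change passes through UpdateStamina, which calls the OnStaminaUsed dispatcher.
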(event `Key|LeftShift`
  (params (Key :type "Key Structure"))
  (bind _charactermovement (`self.CharacterMovement`))
  (:`Pressed`
    (if (not (`self.IsSprinting`))
      (if (> (`self.Stamina`) 0.0) :!label _label
        (set `self.IsSprinting` true)
        (set `CharacterMovementComponent.MaxWalkSpeed` 750.0 _charactermovement)
        (set `self.Stamina` (`KismetMathLibrary.FClamp` (- (`self.Stamina`) 0.05) 0.0 (`self.MaxStamina`)))
        (`self.UpdateStamina`)
        (`KismetSystemLibrary.Delay` 0.5)
        (if (`self.IsSprinting`)
          (goto _label))
        (else
          (set `CharacterMovementComponent.MaxWalkSpeed` 500.0 _charactermovement :!label _label_2)
          (set `self.IsSprinting` false)
          (if (not (== (`self.Stamina`) (`self.MaxStamina`))) :!label _label_3
            (set `self.Stamina` (`KismetMathLibrary.FClamp` (+ (`self.Stamina`) 0.03) 0.0 (`self.MaxStamina`)))
            (`self.UpdateStamina`)
            (`KismetSystemLibrary.Delay` 0.5)
            (if (not (`self.IsSprinting`))
              (goto _label_3)))))))
  (:`Released`
    (goto _label_2)))

(event `UpdateStamina`
  (`self.OnStaminaUsed`))

(fn `UserConstructionScript`)