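; Weapon Blueprint for the X13 gun in the Low Poly Shooter Pack integration, adding a swappable slide/barrel forestock and a reserve magazine to its parent.
; A replicated data table row picks slide and barrel meshes, randomizes with attachments, and receives skin materials.
; The reserve magazine copies the main magazine's mesh and stays hidden until shown through an interface event, usually by animations.
; Grip and scope attach to the rail, whose socket offsets aiming.
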(event `self.ReceiveBeginPlay`
  ;[0.8735 1 0 1 12] Begin Play
  (`parent.ReceiveBeginPlay`)
  (`KismetSystemLibrary.Delay` 0.01)
  (`self.Set Reserve Magazine Visibility` false))

(event `self.On Reload Interrupted`
  ;[0.5468 1 0 1 12] Reload Interrupted Event. Gets called when the reloading animation montage gets interrupted.
  (`parent.On Reload Interrupted`)
  (`self.Set Reserve Magazine Visibility` false))

(event `self.Set Reserve Magazine Visibility`
  (params (Visibility :type Boolean))
  ;[1 0.4522 0 1 12] Set Reserve Magazine Visibility Event. This event gets called when something (usually an animation) is trying to change the visibility of a weapon's reserve magazine.
  (`/Game/InfimaGames/LowPolyShooterPack/Core/Other/BPFL_LPSP_Utility.Update Component Physical Settings` (`self.Magazine Reserve`) (make `/Game/InfimaGames/LowPolyShooterPack/Core/Weapons/Structs/SPhysical` (struct :`Name` "NoCollision") false false Visibility)))

(event `self.On Randomize Attachments`
  ;[0 0.5729 0.0455 1 12] Randomize Attachments Event. Gets called when a character tries to randomize this weapon's attachments.
  (`parent.On Randomize Attachments`)
  (`/Game/InfimaGames/Utilities/Core/BPFL_IG_Utilities_Data_Tables.Randomize Data Table Row Handle Row` (`self.Selected Slide`))
  (set `self.Selected Slide` (`self.Selected Slide`)) ; We have to do this weird hacky thing\nbecause it appears that RepNotifies\ndo not get called when set by ref\nfrom some other place.
)

(event `self.On Equipped`
  ;[0 0.1823 0.00831 1 12] On Equipped Event. Gets called when this weapon gets equipped by a character.
  (`parent.On Equipped`)
  (`KismetSystemLibrary.Delay` 0.01)
  (`self.Set Reserve Magazine Visibility` false))

(fn `Get Extra Aim Offset`
  (returns (Translation :type "Vector Structure"))
  (return (`KismetMathLibrary.NegateVector` (- (.location (`SceneComponent.GetSocketTransform` (`self.Rail`) "SOCKET_Scope" "RTS_Actor")) (.location (`SceneComponent.GetSocketTransform` (`self.Weapon`) "SOCKET_Scope" "RTS_Actor"))))))

(fn `Get Grip Parent`
  (returns (Parent :type "MeshComponent Object Reference"))
  (return (`self.Rail`)))

(fn `Get Muzzle Parent`
  (returns (Parent :type "MeshComponent Object Reference"))
  (return (`self.Barrel`)))

(fn `Get Scope Parent`
  (returns (Parent :type "MeshComponent Object Reference"))
  (return (`self.Rail`)))

(fn `OnRep_Selected Forestock`
  (`self.Update Forestock Mesh`))

(fn `Try Update Attachment Magazine`
  (`parent.Try Update Attachment Magazine`)
  (`StaticMeshComponent.SetStaticMesh` (`self.Magazine Reserve`) (`.Mesh_23_E3ECA4BA4931B1849B8670849EF85707` (break `/Game/InfimaGames/LowPolyShooterPack/Core/Weapons/Structs/SMagazine` (`self.Magazine Settings`)))) ; Copy main magazine mesh over to the\nreserve magazine to make sure that they\nare always the same mesh.
)

(fn `Update Forestock Mesh`
  (bind (_datatable _rowname) (break `DataTableRowHandle` (`self.Selected Slide`)))
  (`|ExecutionSequence`
    (:`then_0`
      (bind _returnvalue (`|GetDataTableRow` _datatable _rowname)
        (:`then`
          (bind _staticmeshes (break `/Game/InfimaGames/LowPolyShooterPack/Core/Weapons/Structs/SMeshes` _returnvalue))
          (`StaticMeshComponent.SetStaticMesh` (`self.Slide`) (`|GetArrayItem` _staticmeshes))
          (`StaticMeshComponent.SetStaticMesh` (`self.Barrel`) (`|GetArrayItem` _staticmeshes 1)))))
    (:`then_1`
      (return))))

(fn `Update Materials From Skin`
  (`parent.Update Materials From Skin`)
  (`/Game/InfimaGames/LowPolyShooterPack/Core/Other/BPFL_LPSP_Utility.Map Materials To Component` (`self.Slide`) (`.MaterialMapBody_36_498E99F74ADF8EB469E4E6A06B3589FC` (break `/Game/InfimaGames/LowPolyShooterPack/Core/Weapons/Structs/SSkin` (`self.Skin`)))) ; Forestock
  (`/Game/InfimaGames/LowPolyShooterPack/Core/Other/BPFL_LPSP_Utility.Map Materials To Component` (`self.Front Ironsights`) (`.MaterialMapIronsights_49_5E36B2744DCF6B7A3D5236BAA5DF8DC4` (break `/Game/InfimaGames/LowPolyShooterPack/Core/Weapons/Structs/SSkin` (`self.Skin`)))) ; Front Ironsight
  (`/Game/InfimaGames/LowPolyShooterPack/Core/Other/BPFL_LPSP_Utility.Map Materials To Component` (`self.Barrel`) (`.MaterialMapBody_36_498E99F74ADF8EB469E4E6A06B3589FC` (break `/Game/InfimaGames/LowPolyShooterPack/Core/Weapons/Structs/SSkin` (`self.Skin`)))) ; Barrel
  (`/Game/InfimaGames/LowPolyShooterPack/Core/Other/BPFL_LPSP_Utility.Map Materials To Component` (`self.Magazine Reserve`) (`.MaterialMapMagazine_41_ED703B284BCCB745316B73AD90D6D688` (break `/Game/InfimaGames/LowPolyShooterPack/Core/Weapons/Structs/SSkin` (`self.Skin`)))) ; Reserve Magazine
)

(fn `UserConstructionScript`
  (`|ExecutionSequence`
    (:`then_0`
      (`self.Update Forestock Mesh`))
    (:`then_1`
      (`parent.UserConstructionScript`)
      (`self.Set Reserve Magazine Visibility` false))))

(fn `Weapon Drop`
  (params (Impulse :type "Vector Structure") (`Angular Impulse` :type "Vector Structure"))
  (`parent.Weapon Drop` Impulse `Angular Impulse`)
  (`self.Set Reserve Magazine Visibility` false))