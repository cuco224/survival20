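; SP60 weapon Blueprint for the Low Poly Shooter Pack integration, extending a parent weapon with a swappable forestock and a reserve magazine.
; A RepNotify forestock data table row sets forestock and barrel meshes, which parent grip and muzzle, and is self-assigned after randomization to trigger the notify.
; The reserve magazine copies the main magazine mesh and is hidden on start, equip, drop and reload interruption.
; Skin updates also cover these extra parts.
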(event `self.ReceiveBeginPlay`
  ;[1 0 0.3351 1 12] Begin Play
  (`parent.ReceiveBeginPlay`)
  (`KismetSystemLibrary.Delay` 0.01)
  (`self.Set Reserve Magazine Visibility` false))

(event `self.Set Reserve Magazine Visibility`
  (params (Visibility :type Boolean))
  ;[1 0.6356 0 1 12] Set Reserve Magazine Visibility Event. This event changes the visibility of the reserve magazine when called.
  (`/Game/InfimaGames/LowPolyShooterPack/Core/Other/BPFL_LPSP_Utility.Update Component Physical Settings` (`self.Magazine Reserve`) (make `/Game/InfimaGames/LowPolyShooterPack/Core/Weapons/Structs/SPhysical` (struct :`Name` "NoCollision") false false Visibility)))

(event `self.On Reload Interrupted`
  ;[0.8014 1 0 1 12] On Reload Interrupted Event. This gets called when the weapon's reload montage gets interrupted by some other montage, or stopped from somewhere.
  (`parent.On Reload Interrupted`)
  (`self.Set Reserve Magazine Visibility` false))

(event `self.On Equipped`
  ;[0.3317 1 0 1 12] On Equipped Event. This event gets called when this weapon gets equipped on a character for the first time.
  (`parent.On Equipped`)
  (`KismetSystemLibrary.Delay` 0.01)
  (`self.Set Reserve Magazine Visibility` false))

(event `self.On Randomize Attachments`
  ;[0.4162 1 0 1 12] Randomize Attachments Event. Gets called when the weapon's attachments are being randomized.
  (`parent.On Randomize Attachments`)
  (`/Game/InfimaGames/Utilities/Core/BPFL_IG_Utilities_Data_Tables.Randomize Data Table Row Handle Row` (`self.Selected Forestock`))
  (set `self.Selected Forestock` (`self.Selected Forestock`)) ; We have to do this weird hacky thing\nbecause it appears that RepNotifies\ndo not get called when set by ref\nfrom some other place.
)

(fn `Get Grip Parent`
  (returns (Parent :type "MeshComponent Object Reference"))
  (return (`self.Forestock`)))

(fn `Get Muzzle Parent`
  (returns (Parent :type "MeshComponent Object Reference"))
  (return (`self.Barrel`)))

(fn `OnRep_Selected Forestock`
  (`|ExecutionSequence`
    (:`then_0`
      (`self.Update Forestock Mesh`))
    (:`then_1`
      (return))))

(fn `Try Update Attachment Magazine`
  (`parent.Try Update Attachment Magazine`)
  (`StaticMeshComponent.SetStaticMesh` (`self.Magazine Reserve`) (`.Mesh_23_E3ECA4BA4931B1849B8670849EF85707` (break `/Game/InfimaGames/LowPolyShooterPack/Core/Weapons/Structs/SMagazine` (`self.Magazine Settings`)))) ; Copy main magazine mesh over to the\nreserve magazine to make sure that they\nare always the same mesh.
)

(fn `Update Forestock Mesh`
  (locals (`Static Meshes` :type "Array of StaticMesh Object Reference"))
  (bind (_datatable _rowname) (break `DataTableRowHandle` (`self.Selected Forestock`)))
  (`|ExecutionSequence`
    (:`then_0`
      (bind _returnvalue (`|GetDataTableRow` _datatable _rowname)
        (:`then`
          (set `local.Static Meshes` (`.StaticMeshes_4_9329442D42053FD2AC0890A1464CC232` (break `/Game/InfimaGames/LowPolyShooterPack/Core/Weapons/Structs/SMeshes` _returnvalue)))
          (`StaticMeshComponent.SetStaticMesh` (`self.Forestock`) (`|GetArrayItem` (`local.Static Meshes`))) ; This updates the forestock mesh with the\nmesh assigned at index zero of the static\nmesh array here.
          (`StaticMeshComponent.SetStaticMesh` (`self.Barrel`) (`|GetArrayItem` (`local.Static Meshes`) 1)) ; This updates the barrel mesh with the\nmesh assigned at index zero of the static\nmesh array here.\n\nWe do this at the same time as the forestock\nbecause these are always paired and have\nto match.
        )))
    (:`then_1`
      (return))))

(fn `Update Materials From Skin`
  (`parent.Update Materials From Skin`)
  (`/Game/InfimaGames/LowPolyShooterPack/Core/Other/BPFL_LPSP_Utility.Map Materials To Component` (`self.Forestock`) (`.MaterialMapBody_36_498E99F74ADF8EB469E4E6A06B3589FC` (break `/Game/InfimaGames/LowPolyShooterPack/Core/Weapons/Structs/SSkin` (`self.Skin`)))) ; Forestock
  (`/Game/InfimaGames/LowPolyShooterPack/Core/Other/BPFL_LPSP_Utility.Map Materials To Component` (`self.Ironsight Front`) (`.MaterialMapIronsights_49_5E36B2744DCF6B7A3D5236BAA5DF8DC4` (break `/Game/InfimaGames/LowPolyShooterPack/Core/Weapons/Structs/SSkin` (`self.Skin`)))) ; Front Ironsight
  (`/Game/InfimaGames/LowPolyShooterPack/Core/Other/BPFL_LPSP_Utility.Map Materials To Component` (`self.Barrel`) (`.MaterialMapBody_36_498E99F74ADF8EB469E4E6A06B3589FC` (break `/Game/InfimaGames/LowPolyShooterPack/Core/Weapons/Structs/SSkin` (`self.Skin`)))) ; Barrel
  (`/Game/InfimaGames/LowPolyShooterPack/Core/Other/BPFL_LPSP_Utility.Map Materials To Component` (`self.Magazine Reserve`) (`.MaterialMapMagazine_41_ED703B284BCCB745316B73AD90D6D688` (break `/Game/InfimaGames/LowPolyShooterPack/Core/Weapons/Structs/SSkin` (`self.Skin`)))) ; Reserve Magazine
)

(fn `UserConstructionScript`
  (`|ExecutionSequence`
    (:`then_0`
      (`self.Update Forestock Mesh`))
    (:`then_1`
      (`parent.UserConstructionScript`)
      (`self.Set Reserve Magazine Visibility` false))))

(fn `Weapon Drop`
  (params (Impulse :type "Vector Structure") (`Angular Impulse` :type "Vector Structure"))
  (`parent.Weapon Drop` Impulse `Angular Impulse`)
  (`self.Set Reserve Magazine Visibility` false))